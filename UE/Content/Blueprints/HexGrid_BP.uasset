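; HexGrid_BP is a grid actor that lays out a hexagonal tile field in its Construction Script.
; It loops over GridX rows along X from GridStartLocation, adding fixed-scale GridTile instances in world space.
; Odd rows shift half a TileWidth along Y and use HexAltValue to drop one tile, forming the staggered pattern.
; Each tile position, plus the GridTile component's world XY, is cached in GridLocations.
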(fn ConstructionScript
  (bind _gridtile (Variables|Default|GetGridTile))
  (bind _gridstartlocation (Variables|Default|GetGridStartLocation))
  (bind _returnvalue (Transformation|GetWorldLocation _gridtile))
  (Utilities|Array|Clear (Variables|Default|GetGridLocations))
  (for _index (range 0 (- (Variables|Default|GetGridX) 1))
    (Variables|Default|SetIsPair? (== (Math|Integer|%(Integer) _index 2) 0))
    (if (== (Math|Integer|%(Integer) _index 2) 0)
      _
      (else
        (Variables|Default|SetHexAltValue 2)))
    (for _index_2 (range 0 (- (Variables|Default|GetGridY) (Variables|Default|GetHexAltValue)))
      (if (Variables|Default|GetIsPair?)
        (Variables|Default|SetYOffset 0)
        (else
          (Variables|Default|SetYOffset (/ (Variables|Default|GetTileWidth) 2))))
      (Components|InstancedStaticMesh|AddInstance (Variables|Default|GetGridTile) (Math|Transform|MakeTransform (Math|Vector|MakeVector (+ (Math|Conversions|ToFloat(Integer) (* _index (Variables|Default|GetTileHeight))) (.x _gridstartlocation)) (+ (+ (.y _gridstartlocation) (Math|Conversions|ToFloat(Integer) (* _index_2 (Variables|Default|GetTileWidth)))) (Variables|Default|GetYOffset)) -25.0) "0, 0, 0" "27.500000,27.500000,27.500000") true)
      (Utilities|Array|Add (Variables|Default|GetGridLocations) (+ (.Location (Math|Transform|BreakTransform (Math|Transform|MakeTransform (Math|Vector|MakeVector (+ (Math|Conversions|ToFloat(Integer) (* _index (Variables|Default|GetTileHeight))) (.x _gridstartlocation)) (+ (+ (.y _gridstartlocation) (Math|Conversions|ToFloat(Integer) (* _index_2 (Variables|Default|GetTileWidth)))) (Variables|Default|GetYOffset)) -25.0) "0, 0, 0" "27.500000,27.500000,27.500000"))) (Math|Vector|MakeVector (.x _returnvalue) (.y _returnvalue) 0.0))))
    (Variables|Default|SetHexAltValue 1)))