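; Game mode for an islands installation driven by serial hardware, with a timeline that moves the ocean water body at start.
; A polled COM port reads start/next commands to step through three phases; Phases 1 and 3 are empty.
; Phase 2 opens a second port and polls distance-sensor lines, which Parser converts into module types by threshold.
; Readings differing from the stored sensor state make Spawner_BP spawn islands at grid positions derived from sensor number.
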(event Custom|Read%20Serial%20Data
  (bind _returnvalue (Class|SerialCom|ReadString (Variables|Default|GetStartNextSerialComRef)))
  (switch string _returnvalue
    (:S
      (CallFunction|Phase1))
    (:N
      (switch int (Variables|Default|GetCurrentPhaseIndex)
        (:1
          (Variables|Default|SetCurrentPhaseIndex 2)
          (CallFunction|Phase2))
        (:2
          (Variables|Default|SetCurrentPhaseIndex 3)
          (CallFunction|Phase3))))))

(event Custom|Phase2
  (Utilities|FlowControl|Sequence
    (:then_0
      (bind _returnvalue (Class|SerialCom|OpenComPort 3 57600))
      (Variables|Default|SetSensorsSerialComRef _returnvalue))
    (:then_1
      (bind _returnvalue_2 (Actor|GetActorOfClass "/Game/Blueprints/Spawner_BP.Spawner_BP_C"))
      (Variables|Default|SetSpawnerRef _returnvalue_2)
      (for _index (range 1 (Variables|Default|GetSensorsCount))
        (Utilities|Array|Add (Variables|Default|GetSensorsState) "NewEnumerator3")))
    (:then_2
      (Utilities|Time|SetTimerbyEvent (delegate Custom|ReadSerialSensorsData) 0.5 true))))

(event Custom|Phase1)

(event Custom|Phase3)

(event Custom|ReadSerialSensorsData
  (bind _spawnerref (Variables|Default|GetSpawnerRef))
  (bind _hexgridreference (Variables|/Game/Blueprints/Spawner_BP.Spawner_BP_C|GetHexGridReference _spawnerref))
  (bind _gridy (Variables|/Game/Blueprints/HexGrid_BP.HexGrid_BP_C|GetGridY _hexgridreference))
  (bind (_bsuccess _returnvalue) (Class|SerialCom|Readln (Variables|Default|GetSensorsSerialComRef)))
  (if _bsuccess
    (bind (_sensornumber _moduletype _isparsingsuccessful_ _isdistancechanged_ _leftover) (CallFunction|Parser _returnvalue))
    (if _isparsingsuccessful_
      (if _isdistancechanged_
        (Default|SpawnIsland (Variables|Default|GetSpawnerRef) _moduletype (Math|Vector2D|MakeVector2D (Math|Conversions|ToFloat(Integer) (/ _sensornumber _gridy)) (Math|Conversions|ToFloat(Integer) (Math|Integer|%(Integer) _gridy _sensornumber))))))))

(event EventEndPlay
  (params (EndPlayReason :type EEndPlayReason%20Enum :default "Destroyed"))
  (Class|SerialCom|Close (Variables|Default|GetSensorsSerialComRef)))

(event EventBeginPlay
  (Utilities|FlowControl|Sequence
    (:then_0
      (bind _returnvalue (Actor|GetActorOfClass "/Script/Water.WaterBodyOcean"))
      (Timeline|Elevate%20Water Play
        (:Update
          (Transformation|SetActorLocation _returnvalue (Math|Vector|Lerp(Vector) "0, 0, 0" "0, 0,1000.000000" 0.0) false false))))
    (:then_1
      (bind _returnvalue_2 (Class|SerialCom|OpenComPort 4 9600))
      (Variables|Default|SetStartNextSerialComRef _returnvalue_2))
    (:then_2
      (Utilities|Time|SetTimerbyEvent (delegate Custom|Read%20Serial%20Data) 0.5 true))))

(fn ConstructionScript)

(fn Parser
  (params (Line :type String))
  (bind (_lefts _rights _returnvalue) (Utilities|String|Split Line ";"))
  (bind (_lefts_2 _rights_2 _returnvalue_2) (Utilities|String|Split _lefts ":"))
  (bind _returnvalue_3 (Math|Conversions|ToInteger(Byte) _lefts_2))
  (bind _returnvalue_4 (Math|Conversions|ToInteger(Byte) _rights_2))
  (if _returnvalue
    _
    (else
      _))
  (if _returnvalue_2
    (if (<= _returnvalue_4 100)
      (LocalVariables|SetCurrentModuleType "NewEnumerator0")
      (elif (<= _returnvalue_4 300)
        (LocalVariables|SetCurrentModuleType "NewEnumerator1")
        (elif (<= _returnvalue_4 500)
          (LocalVariables|SetCurrentModuleType "NewEnumerator2")
          (else
            (LocalVariables|SetCurrentModuleType "NewEnumerator3")))))
    (Variables|Default|SetParsedSensorsCount (+ (Variables|Default|GetParsedSensorsCount) 1))
    (return _returnvalue_3 (LocalVariables|GetCurrentModuleType) true (Utilities|Enum|NotEqual(Enum) (Utilities|Array|Get(acopy) (Variables|Default|GetSensorsState) _returnvalue_3) (LocalVariables|GetCurrentModuleType)) _rights)
    (else
      (return 0 "NewEnumerator0" false false _rights))))

(fn ElevateWater)