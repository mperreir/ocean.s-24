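; Spawner that places island modules on the hex grid, using the HexGrid_BP found at BeginPlay.
; SpawnIsland flattens its Location to a tile index and spawns SampleIsland_BP above that tile for Habitat, Energie or Agricole alike.
; It then removes the grid tile instance, offsetting the index by the deleted count, and records the index in Occupation.
; GetNeighbours is an unfinished stub, and the ControlledElementType assignment and FlattenHexArray formula are unwired.
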(event Custom|Spawn%20Island
  (params (ModuleType :type ModulesEnum_E%20Enum :default "NewEnumerator0") (Location :type Vector%202D%20Structure))
  (bind _returnvalue (Math|Float|Truncate (.x Location)))
  (bind _returnvalue_2 (Math|Float|Truncate (.y Location)))
  (bind _hexgridreference (Variables|Default|GetHexGridReference))
  (bind _zislandoffset (Variables|Default|GetZIslandOffset))
  (bind _index (Utilities|FlattenHexArray _returnvalue _returnvalue_2))
  (bind _gridlocations (Variables|/Game/Blueprints/HexGrid_BP.HexGrid_BP_C|GetGridLocations _hexgridreference))
  (bind _output (Utilities|Array|Get(acopy) _gridlocations _index))
  (bind _returnvalue_3 (+ (.z _output) _zislandoffset))
  (bind _returnvalue_4 (Math|Transform|MakeTransform (Math|Vector|MakeVector (.x _output) (.y _output) _returnvalue_3)))
  (Variables|Default|SetControlledElementIndex _index)
  (switch Utilities|FlowControl|Switch|SwitchonModulesEnum_E ModuleType
    (:NewEnumerator0
      (Game|SpawnActorfromClass "/Game/Blueprints/SampleIsland_BP.SampleIsland_BP_C" _returnvalue_4 "Undefined" 0 0))
    (:NewEnumerator1
      (Game|SpawnActorfromClass "/Game/Blueprints/SampleIsland_BP.SampleIsland_BP_C" _returnvalue_4 "Undefined" 0 0))
    (:NewEnumerator2
      (Game|SpawnActorfromClass "/Game/Blueprints/SampleIsland_BP.SampleIsland_BP_C" _returnvalue_4 "Undefined" 0 0)))
  (Class|InstancedStaticMeshComponent|RemoveInstance (Variables|/Game/Blueprints/HexGrid_BP.HexGrid_BP_C|GetGridTile (Variables|Default|GetHexGridReference)) (- (Variables|Default|GetControlledElementIndex) (Variables|Default|GetDeletedGridTilesCount)))
  (Variables|Default|SetDeletedGridTilesCount (+ (Variables|Default|GetDeletedGridTilesCount) 1))
  (Utilities|Map|Add (Variables|Default|GetOccupation) (Variables|Default|GetControlledElementIndex) (Variables|Default|GetControlledElementType)))

(event EventBeginPlay
  (bind _returnvalue (Actor|GetActorOfClass "/Game/Blueprints/HexGrid_BP.HexGrid_BP_C"))
  (Variables|Default|SetHexGridReference _returnvalue))

(fn ConstructionScript)

(fn GetNeighbours
  (params (X :type Integer) (Y :type Integer))
  (if (and (== X 0) (== Y 0))
    _))